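; Player character Blueprint that holds Health and Herbs values and creates the HUD.
; BeginPlay creates the HUD widget, stores a reference to it and adds it to the viewport.
; Hard-coded number keys lower or raise Health and Herbs in fixed steps, with no clamping.
; The graph never pushes these values to the widget, and overlap, Tick and construction logic are empty.
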(event `Key|Four`
  (params (Key :type "Key Structure" :default "AnyKey"))
  (:`Pressed`
    (set `self.Herbs` (- (`self.Herbs`) 1.0))))

(event `Key|Three`
  (params (Key :type "Key Structure" :default "AnyKey"))
  (:`Pressed`
    (set `self.Herbs` (+ (`self.Herbs`) 1.0))))

(event `Key|Two`
  (params (Key :type "Key Structure" :default "AnyKey"))
  (:`Pressed`
    (set `self.Health` (+ (`self.Health`) 5.0))))

(event `Key|One`
  (params (Key :type "Key Structure" :default "AnyKey"))
  (:`Pressed`
    (set `self.Health` (- (`self.Health`) 5.0))))

(event `self.ReceiveBeginPlay`
  (bind _returnvalue (`|CreateWidget` "/Game/HUD.HUD_C"))
  (bind _output_get (set `self.HUDreference` _returnvalue))
  (`UserWidget.AddToViewport` _output_get 0))

(fn `UserConstructionScript`)